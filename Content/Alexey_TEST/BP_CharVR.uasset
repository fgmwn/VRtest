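; VR character Blueprint with arc teleportation, thumbstick locomotion and object grabbing.
; Holding TeleportRight traces a projectile path each tick and aims an arrow with the right stick; release teleports if the surface is flat enough.
; Grab inputs line-trace from either controller, calling BPI_GrabInterface on one shared held object.
; Movement follows camera vectors flattened horizontally; gamepad turns and pitches, though motion-controller strafe passes zero input.
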(event Custom|Pick%20Up
  (params (AttachHand :type Scene%20Component%20Object%20Reference))
  (bind _returnvalue (Transformation|GetWorldLocation AttachHand))
  ;[1 1 1] Grabbing objects
  (Variables|Default|GetGrabbed
    (:then)
    (:else
      (bind (_outhit _returnvalue_2) (Collision|LineTraceForObjects _returnvalue (+ _returnvalue (* (Math|Vector|GetForwardVector AttachHand) (Variables|Interaction|GetPickUpDistance))) (Utilities|Array|MakeArray "ObjectTypeQuery2") false 0 "ForDuration" true "(R=1.000000,G=0.000000,B=0.000000,A=1.000000)" "(R=0.000000,G=1.000000,B=0.000000,A=1.000000)" 1.0))
      (if _returnvalue_2
        (if (Utilities|DoesObjectImplementInterface (.HitActor (Collision|BreakHitResult _outhit)) "/Game/Alexey_TEST/BPI_GrabInterface.BPI_GrabInterface_C")
          (Class|BPIGrabInterface|GrabActor(Message) (.HitActor (Collision|BreakHitResult _outhit)) AttachHand)
          (Variables|Default|SetGrabbed (.HitActor (Collision|BreakHitResult _outhit))))))))

(event Custom|Drop
  ;[1 1 1] Grabbing objects
  (bind _grabbed (Variables|Default|GetGrabbed)
    (:then
      (Class|BPIGrabInterface|DropActor(Message) _grabbed)
      (Variables|Default|SetGrabbed 0))
    (:else)))

(event EventTick
  (params (DeltaSeconds :type Float%20%28single-precision%29))
  ;[1 1 1] Teleportation
  (if (Variables|Teleportation|GetTeleportKeyPress)
    (CallFunction|TraceforTeleportation)
    (CallFunction|TeleportationRotation)))

(event EventBeginPlay
  ;[1 1 1] Teleportation
  (Transformation|SetWorldScale3D (Variables|Default|GetLeftHand) "1.000000,1.000000,-1.000000")
  (Class|HeadMountedDisplayFunctionLibrary|SetTrackingOrigin "Floor"))

(event Input|ActionEvents|InputActionTeleportRight
  (params (Key :type Key%20Structure :default "None"))
  (bind _returnvalue (Pawn|GetControlRotation :!class /Script/Engine.Pawn))
  ;[1 1 1] Teleportation
  (:Pressed
    (Variables|Teleportation|SetTeleportKeyPress true))
  (:Released
    (Variables|Teleportation|SetTeleportKeyPress false)
    (Development|SetHiddeninGame (Variables|Default|GetTeleportationRotationArrow) true false)
    (if (Variables|Teleportation|GetCanTeleport)
      (Transformation|Teleport (Variables|Teleportation|GetTeleportLocation) (Math|Rotator|MakeRotator 0.0 0.0 (.yaw (Math|Rotator|CombineRotators (Math|Rotator|Delta(Rotator) (Transformation|GetWorldRotation (Variables|Default|GetTeleportationRotationArrow)) _returnvalue) _returnvalue)))))))

(event Input|ActionEvents|InputActionGrabLeft
  (params (Key :type Key%20Structure :default "None"))
  ;[1 1 1] Left
  (:Pressed
    (CallFunction|PickUp (Variables|Default|GetLeftMC)))
  (:Released
    (CallFunction|Drop)))

(event Input|ActionEvents|InputActionGrabRight
  (params (Key :type Key%20Structure :default "None"))
  ;[1 1 1] Input for pick ups and drops
  (:Pressed
    (CallFunction|PickUp (Variables|Default|GetRightMC)))
  (:Released
    (CallFunction|Drop)))

(event Input|MouseEvents|RightMouseButton
  (params (Key :type Key%20Structure :default "None"))
  ;[1 1 1] Input for pick ups and drops
  (:Pressed
    (CallFunction|PickUp (Variables|Default|GetRightMC)))
  (:Released
    (CallFunction|Drop)))

(event Input|AxisEvents|InputAxisMotionControllerThumbLeft_X
  (params (AxisValue :type Float%20%28single-precision%29))
  ;[1 1 1] Side Movement
  (if (not (== AxisValue 0.0))
    (CallFunction|HandleMovement 0.0 (Math|Vector|GetRightVector (Variables|Default|GetCamera)))))

(event Input|AxisEvents|InputAxisMotionControllerThumbLeft_Y
  (params (AxisValue :type Float%20%28single-precision%29))
  ;[1 1 1] Forward Movement
  (if (not (== AxisValue 0.0))
    (CallFunction|HandleMovement AxisValue (Math|Vector|GetForwardVector (Variables|Default|GetCamera)))))

(event Input|GamepadEvents|GamepadRightX
  (params (AxisValue :type Float%20%28single-precision%29))
  ;[1 1 1] Rotation
  (if (> (Math|Float|Absolute(Float) AxisValue) (Variables|Movement|GetRotationDeadZone))
    (Class|Actor|AddActorWorldRotation (Math|Rotator|MakeRotator 0.0 0.0 (select (> AxisValue 0.0) 1.0 -1.0)))))

(event Input|GamepadEvents|GamepadLeftY
  (params (AxisValue :type Float%20%28single-precision%29))
  ;[1 1 1] Forward Movement
  (if (not (== AxisValue 0.0))
    (CallFunction|HandleMovement AxisValue (Math|Vector|GetForwardVector (Variables|Default|GetCamera)))))

(event Input|GamepadEvents|GamepadLeftX
  (params (AxisValue :type Float%20%28single-precision%29))
  ;[1 1 1] Side Movement
  (if (not (== AxisValue 0.0))
    (CallFunction|HandleMovement AxisValue (Math|Vector|GetRightVector (Variables|Default|GetCamera)))))

(event Input|GamepadEvents|GamepadRightY
  (params (AxisValue :type Float%20%28single-precision%29))
  ;[1 1 1] Rotation
  (if (> (Math|Float|Absolute(Float) AxisValue) (Variables|Movement|GetRotationDeadZone))
    (Transformation|AddRelativeRotation (Variables|Default|GetCamera) (Math|Rotator|MakeRotator 0.0 (select (> AxisValue 0.0) 1.0 -1.0) 0.0) false false)))

(fn ConstructionScript)

(fn TraceforTeleportation
  (bind _rightmc (Variables|Default|GetRightMC))
  (bind _teleportationrotationarrow (Variables|Default|GetTeleportationRotationArrow))
  (bind (_outhit _outpathpositions _outlasttracedestination _returnvalue) (Class|GameplayStatics|BlueprintPredictProjectilePathbyObjectType (Transformation|GetWorldLocation _rightmc) (* (Math|Vector|GetForwardVector (Transformation|GetWorldRotation _rightmc)) (Variables|Teleportation|GetTeleportationTraceLength)) true 1e+01 (Utilities|Array|MakeArray "ObjectTypeQuery1" "ObjectTypeQuery2") false 0 "ForOneFrame" 0.0 2e+01))
  (if _returnvalue
    (Variables|Teleportation|SetCanTeleport (> (.Z (Math|Vector|BreakVector (.ImpactNormal (Collision|BreakHitResult _outhit)))) 0.5))
    (bind _output_get (Variables|Teleportation|SetTeleportLocation (.ImpactPoint (Collision|BreakHitResult _outhit))))
    (Class|KismetSystemLibrary|DrawDebugCylinder _output_get (+ _output_get "0, 0,20.000000") 5e+01 20 "(R=0.000000,G=0.164047,B=1.000000,A=1.000000)" 0.0 0.0)
    (Development|SetHiddeninGame _teleportationrotationarrow false false)
    (Transformation|SetWorldLocation _teleportationrotationarrow (Variables|Teleportation|GetTeleportLocation) false false)
    (else
      (Development|SetHiddeninGame (Variables|Default|GetTeleportationRotationArrow) true false)
      (Variables|Teleportation|SetCanTeleport false))))

(fn TeleportationRotation
  (Transformation|SetWorldRotation (Variables|Default|GetTeleportationRotationArrow) (Math|Rotator|MakeRotator 0.0 0.0 (.yaw (Math|Rotator|CombineRotators (Math|Conversions|RotationFromXVector (Math|Vector|MakeVector (Input|AxisValues|GetMotionControllerThumbRight_Y) (Input|AxisValues|GetMotionControllerThumbRight_X) 0.0)) (Transformation|GetWorldRotation (Variables|Default|GetRightMC))))) false false))

(fn HandleMovement
  (params (InAxisValue :type Float%20%28single-precision%29) (InVector :type Vector))
  (bind (_x _y) (Math|Vector|BreakVector InVector))
  (Pawn|Input|AddMovementInput (Math|Vector|MakeVector _x _y 0.0) (* InAxisValue (Variables|Movement|GetMovementSpeed)) false))